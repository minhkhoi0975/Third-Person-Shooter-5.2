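; Procedural mesh Blueprint that defines a cone from Height, Radius and Resolution, extending a parent class's construction script.
; GenerateVerticesAndTriangles creates two center points and a rotated base ring, then links them into side and bottom triangles with wrapped indices.
; ProcessVertices expands these into unshared per-triangle vertices with sequential indices.
; ProcessUV repeats a fixed triangular UV layout for each side and bottom pair.
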(event EventProcessUV
  (Utilities|Array|Clear (Variables|Default|GetRealUVs))
  (for _index (range 1 (/ (Utilities|Array|Length (Variables|Default|GetRealVertices)) 6))
    ;[1 1 1] Side Triangle
    (Utilities|Array|Add :TargetArray (Variables|Default|GetRealUVs))
    (Utilities|Array|Add (Variables|Default|GetRealUVs) "(X=0.500000,Y=1.000000)")
    (Utilities|Array|Add (Variables|Default|GetRealUVs) "(X=1.000000,Y=0.000000)")
    ;[1 1 1] Bottom Triangle
    (Utilities|Array|Add (Variables|Default|GetRealUVs) "(X=0.000000,Y=0.000000)")
    (Utilities|Array|Add (Variables|Default|GetRealUVs) "(X=0.500000,Y=1.000000)")
    (Utilities|Array|Add (Variables|Default|GetRealUVs) "(X=1.000000,Y=0.000000)")))

(event EventProcessVertices
  (Utilities|Array|Clear (Variables|Default|GetRealVertices))
  (Utilities|Array|Clear (Variables|Default|GetRealTriangles))
  (bind (_unique_vertices _triangles) (CallFunction|GenerateVerticesandTriangles))
  (for (_ _array_index) _triangles
    (Utilities|Array|Add (Variables|Default|GetRealVertices) (Utilities|Array|Get(acopy) _unique_vertices (Utilities|Array|Get(acopy) _triangles _array_index))))
  (for (_ _array_index_2) (Variables|Default|GetRealVertices)
    (Utilities|Array|Add (Variables|Default|GetRealTriangles) _array_index_2)))

(fn ConstructionScript
  (|CallParentFunction))

(fn GenerateVerticesandTriangles
  (bind _m_uniquevertices (LocalVariables|Getm_UniqueVertices))
  (Utilities|Array|Clear (LocalVariables|Getm_UniqueVertices))
  (Utilities|Array|Clear (LocalVariables|Getm_Triangles))
  (Utilities|FlowControl|Sequence
    (:then_0
      ;[1 1 1] Generate Vertices
      ;;[1 1 1] Generate central vertices
      ;;;[1 1 1] Bottom
      (Utilities|Array|Add :TargetArray _m_uniquevertices)
      ;;;[1 1 1] Top
      (Utilities|Array|Add _m_uniquevertices (Math|Vector|MakeVector 0.0 0.0 (Variables|ProceduralMesh|GetHeight)))
      ;;[1 1 1] Generate side vertices
      (LocalVariables|SetcentralAngle (/ 3.6e+02 (Math|Conversions|ToFloat(Integer) (Variables|ProceduralMesh|GetResolution))))
      (for _index (range 0 (- (Variables|ProceduralMesh|GetResolution) 1))
        ;;;[1 1 1] 2D location
        (bind _output_get (LocalVariables|Setvertex2D (Math|Vector2D|MakeVector2D 0.0 (Variables|ProceduralMesh|GetRadius))))
        (bind _output_get_2 (LocalVariables|Setvertex2D (Class|KismetMathLibrary|GetRotated2D _output_get (* (LocalVariables|GetcentralAngle) (Math|Conversions|ToFloat(Integer) _index)))))
        ;;;[1 1 1] Bottom
        (Utilities|Array|Add (LocalVariables|Getm_UniqueVertices) (Math|Vector|MakeVector (.x _output_get_2) (.y _output_get_2) 0.0))))
    (:then_1
      ;[1 1 1] Generate triangles
      (for _index_2 (range 0 (- (Variables|ProceduralMesh|GetResolution) 1))
        ;;[1 1 1] Side triangle
        (Utilities|Array|Add (LocalVariables|Getm_Triangles) (|(2+((index+1)%{DFA98BFE-49E7-D2E3-928D-479A2DBB19DD})) _index_2))
        (Utilities|Array|Add (LocalVariables|Getm_Triangles) 0)
        (Utilities|Array|Add (LocalVariables|Getm_Triangles) (|(index+2) _index_2))
        ;;[1 1 1] Bottom triangle
        (Utilities|Array|Add (LocalVariables|Getm_Triangles) (|(index+2) _index_2))
        (Utilities|Array|Add (LocalVariables|Getm_Triangles) 1)
        (Utilities|Array|Add (LocalVariables|Getm_Triangles) (|(2+((index+1)%{DFA98BFE-49E7-D2E3-928D-479A2DBB19DD})) _index_2))))
    (:then_2
      (return (LocalVariables|Getm_UniqueVertices) (LocalVariables|Getm_Triangles)))))