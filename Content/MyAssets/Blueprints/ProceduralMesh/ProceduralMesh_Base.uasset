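; Base Blueprint for procedural meshes, with empty ProcessVertices, ProcessTriangles and ProcessUV events as hooks for filling the geometry arrays.
; The construction script calls those hooks, calculates normals, then creates the mesh section with optional collision and applies the material.
; CalculateNormals gives flat per-face normals via cross products, reading vertices as consecutive unshared triples rather than through triangle indices.
; ReconstructMesh clears the arrays and repeats the build.
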(event Custom|Process%20Triangles)

(event Custom|Process%20Vertices)

(event Custom|Process%20UV)

(fn ConstructionScript
  (bind _mesh (Variables|Default|GetMesh))
  (CallFunction|ProcessVertices)
  (CallFunction|ProcessTriangles)
  (CallFunction|ProcessUV)
  (CallFunction|CalculateNormals)
  (Class|ProceduralMeshComponent|CreateMeshSectionLinearColor _mesh 0 (Variables|ProceduralMesh|GetRealVertices) (Variables|ProceduralMesh|GetRealTriangles) (Variables|ProceduralMesh|GetRealNormals) (Variables|ProceduralMesh|GetRealUVs) 0 0 0 0 0 (Variables|ProceduralMesh|GetCollision) false)
  (Rendering|Material|SetMaterial _mesh 0 (Variables|ProceduralMesh|GetMaterial)))

(fn CalculateNormals
  (bind _realvertices (Variables|ProceduralMesh|GetRealVertices))
  (for _index (range 0 (- (/ (Utilities|Array|Length (Variables|ProceduralMesh|GetRealTriangles)) 3) 1))
    (for _index_2 (range 0 2)
      (Utilities|Array|Add (Variables|ProceduralMesh|GetRealNormals) (Math|Vector|Normalize (Math|Vector|CrossProduct (- (Utilities|Array|Get(acopy) _realvertices (|((3*index)+1) _index)) (Utilities|Array|Get(acopy) _realvertices (|(3*index) _index))) (- (Utilities|Array|Get(acopy) _realvertices (|((3*index)+1) _index)) (Utilities|Array|Get(acopy) _realvertices (|((3*index)+2) _index)))))))))

(fn ReconstructMesh
  (bind _mesh (Variables|Default|GetMesh))
  (Utilities|Array|Clear (Variables|ProceduralMesh|GetRealVertices))
  (Utilities|Array|Clear (Variables|ProceduralMesh|GetRealTriangles))
  (Utilities|Array|Clear (Variables|ProceduralMesh|GetRealUVs))
  (Utilities|Array|Clear (Variables|ProceduralMesh|GetRealNormals))
  (CallFunction|ProcessVertices)
  (CallFunction|ProcessTriangles)
  (CallFunction|ProcessUV)
  (CallFunction|CalculateNormals)
  (Class|ProceduralMeshComponent|CreateMeshSectionLinearColor _mesh 0 (Variables|ProceduralMesh|GetRealVertices) (Variables|ProceduralMesh|GetRealTriangles) (Variables|ProceduralMesh|GetRealNormals) (Variables|ProceduralMesh|GetRealUVs) 0 0 0 0 0 (Variables|ProceduralMesh|GetCollision) false)
  (Rendering|Material|SetMaterial _mesh 0 (Variables|ProceduralMesh|GetMaterial)))