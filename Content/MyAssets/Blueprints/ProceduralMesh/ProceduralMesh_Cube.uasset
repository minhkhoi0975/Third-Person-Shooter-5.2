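; Procedural box mesh Blueprint that builds cube geometry from a Size vector, with one corner at the local origin.
; GenerateVerticesAndTriangles defines eight shared corners and the triangle indices for six quads.
; ProcessVertices expands these into unshared per-triangle vertices with sequential indices, so ProcessUV can give every face the same unit-square UV layout.
; The construction script only calls the parent, and no mesh section is created in this file.
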(event `self.Process Vertices`
  (`KismetArrayLibrary.Array_Clear` (`self.RealVertices`))
  (`KismetArrayLibrary.Array_Clear` (`self.RealTriangles`))
  (bind (_unique_vertices _triangles) (`self.GenerateVerticesAndTriangles`))
  (for (_ _array_index) _triangles
    (`KismetArrayLibrary.Array_Add` (`self.RealVertices`) (`|GetArrayItem` _unique_vertices (`|GetArrayItem` _triangles _array_index))))
  (for (_ _array_index_2) (`self.RealVertices`)
    (`KismetArrayLibrary.Array_Add` (`self.RealTriangles`) _array_index_2)))

(event `self.Process UV`
  (`KismetArrayLibrary.Array_Clear` (`self.RealUVs`))
  (`|ExecutionSequence`
    (:`then_0`
      ;[1 1 1] Apply UVs to 6 quads
      (for _ (range 6)
        (`KismetArrayLibrary.Array_Add` (`self.RealUVs`))
        (`KismetArrayLibrary.Array_Add` (`self.RealUVs`) (0.0 1.0))
        (`KismetArrayLibrary.Array_Add` (`self.RealUVs`) (1.0 1.0))
        (`KismetArrayLibrary.Array_Add` (`self.RealUVs`))
        (`KismetArrayLibrary.Array_Add` (`self.RealUVs`) (1.0 1.0))
        (`KismetArrayLibrary.Array_Add` (`self.RealUVs`) (1.0 0.0))))))

(fn `GenerateVerticesAndTriangles`
  (returns (`Unique Vertices` :type "Array of Vector Structure") (Triangles :type "Array of Integer"))
  (locals (m_UniqueVertices :type "Array of Vector Structure") (m_Triangles :type "Array of Integer"))
  (bind _m_uniquevertices (`local.m_UniqueVertices`))
  (bind (_size_x _size_y _size_z) (`KismetMathLibrary.BreakVector` (`self.Size`)))
  (`KismetArrayLibrary.Array_Clear` (`local.m_UniqueVertices`))
  (`KismetArrayLibrary.Array_Clear` (`local.m_Triangles`))
  (`|ExecutionSequence`
    (:`then_0`
      ;[1 1 1] Generate Vertices
      (`KismetArrayLibrary.Array_Add` _m_uniquevertices)
      (`KismetArrayLibrary.Array_Add` _m_uniquevertices (`KismetMathLibrary.MakeVector` _size_x))
      (`KismetArrayLibrary.Array_Add` _m_uniquevertices (`KismetMathLibrary.MakeVector` _size_x _size_y))
      (`KismetArrayLibrary.Array_Add` _m_uniquevertices (`KismetMathLibrary.MakeVector` 0.0 _size_y))
      (`KismetArrayLibrary.Array_Add` _m_uniquevertices (`KismetMathLibrary.MakeVector` 0.0 0.0 _size_z))
      (`KismetArrayLibrary.Array_Add` _m_uniquevertices (`KismetMathLibrary.MakeVector` _size_x 0.0 _size_z))
      (`KismetArrayLibrary.Array_Add` _m_uniquevertices (`KismetMathLibrary.MakeVector` _size_x _size_y _size_z))
      (`KismetArrayLibrary.Array_Add` _m_uniquevertices (`KismetMathLibrary.MakeVector` 0.0 _size_y _size_z)))
    (:`then_1`
      ;[1 1 1] Generate triangles
      (`|ExecutionSequence`
        (:`then_0`
          ;;[1 1 1] Bottom Quad
          (`KismetArrayLibrary.Array_Add` (`local.m_Triangles`))
          (`KismetArrayLibrary.Array_Add` (`local.m_Triangles`) 1)
          (`KismetArrayLibrary.Array_Add` (`local.m_Triangles`) 2)
          (`KismetArrayLibrary.Array_Add` (`local.m_Triangles`))
          (`KismetArrayLibrary.Array_Add` (`local.m_Triangles`) 2)
          (`KismetArrayLibrary.Array_Add` (`local.m_Triangles`) 3))
        (:`then_1`
          ;;[1 1 1] Top Quad
          (`KismetArrayLibrary.Array_Add` (`local.m_Triangles`) 4)
          (`KismetArrayLibrary.Array_Add` (`local.m_Triangles`) 7)
          (`KismetArrayLibrary.Array_Add` (`local.m_Triangles`) 6)
          (`KismetArrayLibrary.Array_Add` (`local.m_Triangles`) 4)
          (`KismetArrayLibrary.Array_Add` (`local.m_Triangles`) 6)
          (`KismetArrayLibrary.Array_Add` (`local.m_Triangles`) 5))
        (:`then_2`
          ;;[1 1 1] Front Quad
          (`KismetArrayLibrary.Array_Add` (`local.m_Triangles`))
          (`KismetArrayLibrary.Array_Add` (`local.m_Triangles`) 4)
          (`KismetArrayLibrary.Array_Add` (`local.m_Triangles`) 5)
          (`KismetArrayLibrary.Array_Add` (`local.m_Triangles`))
          (`KismetArrayLibrary.Array_Add` (`local.m_Triangles`) 5)
          (`KismetArrayLibrary.Array_Add` (`local.m_Triangles`) 1))
        (:`then_3`
          ;;[1 1 1] Back Quad
          (`KismetArrayLibrary.Array_Add` (`local.m_Triangles`) 2)
          (`KismetArrayLibrary.Array_Add` (`local.m_Triangles`) 6)
          (`KismetArrayLibrary.Array_Add` (`local.m_Triangles`) 7)
          (`KismetArrayLibrary.Array_Add` (`local.m_Triangles`) 2)
          (`KismetArrayLibrary.Array_Add` (`local.m_Triangles`) 7)
          (`KismetArrayLibrary.Array_Add` (`local.m_Triangles`) 3))
        (:`then_4`
          ;;[1 1 1] Left Quad
          (`KismetArrayLibrary.Array_Add` (`local.m_Triangles`) 3)
          (`KismetArrayLibrary.Array_Add` (`local.m_Triangles`) 7)
          (`KismetArrayLibrary.Array_Add` (`local.m_Triangles`) 4)
          (`KismetArrayLibrary.Array_Add` (`local.m_Triangles`) 3)
          (`KismetArrayLibrary.Array_Add` (`local.m_Triangles`) 4)
          (`KismetArrayLibrary.Array_Add` (`local.m_Triangles`)))
        (:`then_5`
          ;;[1 1 1] Right Quad
          (`KismetArrayLibrary.Array_Add` (`local.m_Triangles`) 1)
          (`KismetArrayLibrary.Array_Add` (`local.m_Triangles`) 5)
          (`KismetArrayLibrary.Array_Add` (`local.m_Triangles`) 6)
          (`KismetArrayLibrary.Array_Add` (`local.m_Triangles`) 1)
          (`KismetArrayLibrary.Array_Add` (`local.m_Triangles`) 6)
          (`KismetArrayLibrary.Array_Add` (`local.m_Triangles`) 2))))
    (:`then_2`
      (return (`local.m_UniqueVertices`) (`local.m_Triangles`)))))

(fn `UserConstructionScript`
  (`parent.UserConstructionScript`))