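; Procedural mesh Blueprint that supplies the geometry of a wedge-shaped ramp scaled by Size, rising along Y to full Z height.
; GenerateVerticesAndTriangles defines six corner points and indexes them into three quads and two side triangles.
; ProcessVertices expands these into unshared per-triangle vertices with sequential indices, so ProcessUV can map each face separately in the same order.
; The construction script defers to the parent class.
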(event `self.Process Vertices`
  (`KismetArrayLibrary.Array_Clear` (`self.RealVertices`))
  (`KismetArrayLibrary.Array_Clear` (`self.RealTriangles`))
  (bind (_unique_vertices _triangles) (`self.GenerateVerticesAndTriangles`))
  (for (_ _array_index) _triangles
    (`KismetArrayLibrary.Array_Add` (`self.RealVertices`) (`|GetArrayItem` _unique_vertices (`|GetArrayItem` _triangles _array_index))))
  (for (_ _array_index_2) (`self.RealVertices`)
    (`KismetArrayLibrary.Array_Add` (`self.RealTriangles`) _array_index_2)))

(event `self.Process UV`
  (`KismetArrayLibrary.Array_Clear` (`self.RealUVs`))
  (`|ExecutionSequence`
    (:`then_0`
      ;[1 1 1] Apply UVs to 3 quads
      (for _ (range 3)
        (`KismetArrayLibrary.Array_Add` (`self.RealUVs`))
        (`KismetArrayLibrary.Array_Add` (`self.RealUVs`) (0.0 1.0))
        (`KismetArrayLibrary.Array_Add` (`self.RealUVs`) (1.0 1.0))
        (`KismetArrayLibrary.Array_Add` (`self.RealUVs`))
        (`KismetArrayLibrary.Array_Add` (`self.RealUVs`) (1.0 1.0))
        (`KismetArrayLibrary.Array_Add` (`self.RealUVs`) (1.0 0.0))))
    (:`then_1`
      ;[1 1 1] Apply UVs to 2 side traingles
      (`KismetArrayLibrary.Array_Add` (`self.RealUVs`))
      (`KismetArrayLibrary.Array_Add` (`self.RealUVs`) (0.0 1.0))
      (`KismetArrayLibrary.Array_Add` (`self.RealUVs`) (1.0 0.0))
      (`KismetArrayLibrary.Array_Add` (`self.RealUVs`))
      (`KismetArrayLibrary.Array_Add` (`self.RealUVs`) (1.0 1.0))
      (`KismetArrayLibrary.Array_Add` (`self.RealUVs`) (1.0 0.0)))))

(fn `GenerateVerticesAndTriangles`
  (returns (`Unique Vertices` :type "Array of Vector Structure") (Triangles :type "Array of Integer"))
  (locals (m_UniqueVertices :type "Array of Vector Structure") (m_Triangles :type "Array of Integer"))
  (`KismetArrayLibrary.Array_Clear` (`local.m_UniqueVertices`))
  (`KismetArrayLibrary.Array_Clear` (`local.m_Triangles`))
  (`|ExecutionSequence`
    (:`then_0`
      ;[1 1 1] Generate Vertices
      (`KismetArrayLibrary.Array_Add` (`local.m_UniqueVertices`))
      (`KismetArrayLibrary.Array_Add` (`local.m_UniqueVertices`) (`KismetMathLibrary.MakeVector` 0.0 (.y (`self.Size`)) (.z (`self.Size`))))
      (`KismetArrayLibrary.Array_Add` (`local.m_UniqueVertices`) (`KismetMathLibrary.MakeVector` (.x (`self.Size`)) (.y (`self.Size`)) (.z (`self.Size`))))
      (`KismetArrayLibrary.Array_Add` (`local.m_UniqueVertices`) (`KismetMathLibrary.MakeVector` (.x (`self.Size`))))
      (`KismetArrayLibrary.Array_Add` (`local.m_UniqueVertices`) (`KismetMathLibrary.MakeVector` 0.0 (.y (`self.Size`))))
      (`KismetArrayLibrary.Array_Add` (`local.m_UniqueVertices`) (`KismetMathLibrary.MakeVector` (.x (`self.Size`)) (.y (`self.Size`)))))
    (:`then_1`
      ;[1 1 1] Generate triangles
      ;;[1 1 1] Ramp quad
      (`KismetArrayLibrary.Array_Add` (`local.m_Triangles`))
      (`KismetArrayLibrary.Array_Add` (`local.m_Triangles`) 1)
      (`KismetArrayLibrary.Array_Add` (`local.m_Triangles`) 2)
      (`KismetArrayLibrary.Array_Add` (`local.m_Triangles`))
      (`KismetArrayLibrary.Array_Add` (`local.m_Triangles`) 2)
      (`KismetArrayLibrary.Array_Add` (`local.m_Triangles`) 3))
    (:`then_2`
      ;;[1 1 1] Back quad
      (`KismetArrayLibrary.Array_Add` (`local.m_Triangles`) 5)
      (`KismetArrayLibrary.Array_Add` (`local.m_Triangles`) 2)
      (`KismetArrayLibrary.Array_Add` (`local.m_Triangles`) 1)
      (`KismetArrayLibrary.Array_Add` (`local.m_Triangles`) 5)
      (`KismetArrayLibrary.Array_Add` (`local.m_Triangles`) 1)
      (`KismetArrayLibrary.Array_Add` (`local.m_Triangles`) 4))
    (:`then_3`
      ;;[1 1 1] Bottom quad
      (`KismetArrayLibrary.Array_Add` (`local.m_Triangles`) 3)
      (`KismetArrayLibrary.Array_Add` (`local.m_Triangles`) 5)
      (`KismetArrayLibrary.Array_Add` (`local.m_Triangles`) 4)
      (`KismetArrayLibrary.Array_Add` (`local.m_Triangles`) 3)
      (`KismetArrayLibrary.Array_Add` (`local.m_Triangles`) 4)
      (`KismetArrayLibrary.Array_Add` (`local.m_Triangles`)))
    (:`then_4`
      ;;[1 1 1] Side triangles
      (`KismetArrayLibrary.Array_Add` (`local.m_Triangles`) 4)
      (`KismetArrayLibrary.Array_Add` (`local.m_Triangles`) 1)
      (`KismetArrayLibrary.Array_Add` (`local.m_Triangles`))
      (`KismetArrayLibrary.Array_Add` (`local.m_Triangles`) 3)
      (`KismetArrayLibrary.Array_Add` (`local.m_Triangles`) 2)
      (`KismetArrayLibrary.Array_Add` (`local.m_Triangles`) 5))
    (:`then_5`
      (return (`local.m_UniqueVertices`) (`local.m_Triangles`)))))

(fn `UserConstructionScript`
  (`parent.UserConstructionScript`))