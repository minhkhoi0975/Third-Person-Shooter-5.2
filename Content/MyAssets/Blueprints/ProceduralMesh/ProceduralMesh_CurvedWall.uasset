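; Procedural mesh Blueprint for a curved wall: a block of given Size with a concave quarter-circle cut of given Radius at one corner.
; GenerateVerticesAndTriangles rotates a point in Resolution steps to trace the arc, then builds top, bottom and side faces.
; ProcessVertices expands these into unshared vertices per triangle, with sequential indices.
; ProcessUV only clears RealUVs; its per-face UV fill is disconnected.
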(event EventProcessUV
  (Utilities|Array|Clear (Variables|Default|GetRealUVs)))

(event EventProcessVertices
  (Utilities|Array|Clear (Variables|Default|GetRealVertices))
  (Utilities|Array|Clear (Variables|Default|GetRealTriangles))
  (bind (_unique_vertices _triangles) (CallFunction|GenerateVerticesandTriangles))
  (for (_ _array_index) _triangles
    (Utilities|Array|Add (Variables|Default|GetRealVertices) (Utilities|Array|Get(acopy) _unique_vertices (Utilities|Array|Get(acopy) _triangles _array_index))))
  (for (_ _array_index_2) (Variables|Default|GetRealVertices)
    (Utilities|Array|Add (Variables|Default|GetRealTriangles) _array_index_2)))

(fn ConstructionScript
  (|CallParentFunction))

(fn GenerateVerticesandTriangles
  (bind _size (Variables|ProceduralMesh|GetSize))
  (bind _size_2 (Variables|ProceduralMesh|GetSize))
  (bind _size_3 (Variables|ProceduralMesh|GetSize))
  (bind _returnvalue (Math|Vector2D|MakeVector2D (.x _size_2) (.y _size_2)))
  (Utilities|Array|Clear (LocalVariables|Getm_UniqueVertices))
  (Utilities|Array|Clear (LocalVariables|Getm_Triangles))
  (Utilities|FlowControl|Sequence
    (:then_0
      ;[1 1 1] Generate Vertices
      (Utilities|FlowControl|Sequence
        (:then_0
          (LocalVariables|SetTheta (/ 9e+01 (Math|Conversions|ToFloat(Integer) (Variables|ProceduralMesh|GetResolution)))))
        (:then_1
          (Utilities|Array|Add :TargetArray (LocalVariables|Getm_UniqueVertices))
          (Utilities|Array|Add (LocalVariables|Getm_UniqueVertices) (Math|Vector|MakeVector 0.0 0.0 (.z (Variables|ProceduralMesh|GetSize)))))
        (:then_2
          (Utilities|Array|Add (LocalVariables|Getm_UniqueVertices) (Math|Vector|MakeVector (.x (Variables|ProceduralMesh|GetSize)) 0.0 0.0))
          (Utilities|Array|Add (LocalVariables|Getm_UniqueVertices) (Math|Vector|MakeVector (.x _size) 0.0 (.z _size))))
        (:then_3
          (for _index (range 0 (Variables|ProceduralMesh|GetResolution))
            (Utilities|Array|Add (LocalVariables|Getm_UniqueVertices) (Math|Vector|MakeVector (.x (+ (Class|KismetMathLibrary|GetRotated2D (- (Math|Vector2D|MakeVector2D (.x _size_2) (- (.y _size_2) (Variables|ProceduralMesh|GetRadius))) _returnvalue) (* _index (- 0.0 (LocalVariables|GetTheta)))) _returnvalue)) (.y (+ (Class|KismetMathLibrary|GetRotated2D (- (Math|Vector2D|MakeVector2D (.x _size_2) (- (.y _size_2) (Variables|ProceduralMesh|GetRadius))) _returnvalue) (* _index (- 0.0 (LocalVariables|GetTheta)))) _returnvalue)) 0.0))
            (Utilities|Array|Add (LocalVariables|Getm_UniqueVertices) (Math|Vector|MakeVector (.x (+ (Class|KismetMathLibrary|GetRotated2D (- (Math|Vector2D|MakeVector2D (.x _size_2) (- (.y _size_2) (Variables|ProceduralMesh|GetRadius))) _returnvalue) (* _index (- 0.0 (LocalVariables|GetTheta)))) _returnvalue)) (.y (+ (Class|KismetMathLibrary|GetRotated2D (- (Math|Vector2D|MakeVector2D (.x _size_2) (- (.y _size_2) (Variables|ProceduralMesh|GetRadius))) _returnvalue) (* _index (- 0.0 (LocalVariables|GetTheta)))) _returnvalue)) (.z (Variables|ProceduralMesh|GetSize))))))
        (:then_4
          (Utilities|Array|Add (LocalVariables|Getm_UniqueVertices) (Math|Vector|MakeVector 0.0 (.y (Variables|ProceduralMesh|GetSize)) 0.0))
          (Utilities|Array|Add (LocalVariables|Getm_UniqueVertices) (Math|Vector|MakeVector 0.0 (.y _size_3) (.z _size_3))))))
    (:then_1
      ;[1 1 1] Generate triangles
      (Utilities|FlowControl|Sequence
        (:then_0
          ;;[1 1 1] Curve Bottom
          (for _index_2 (range 1 (+ (Variables|ProceduralMesh|GetResolution) 2))
            (Utilities|Array|Add (LocalVariables|Getm_Triangles) (* _index_2 2))
            (Utilities|Array|Add (LocalVariables|Getm_Triangles) (|((2*index)+2) _index_2))
            (Utilities|Array|Add (LocalVariables|Getm_Triangles) 0)))
        (:then_1
          ;;[1 1 1] Curve Top
          (for _index_3 (range 1 (+ (Variables|ProceduralMesh|GetResolution) 2))
            (Utilities|Array|Add (LocalVariables|Getm_Triangles) 1)
            (Utilities|Array|Add (LocalVariables|Getm_Triangles) (|((2*index)+3) _index_3))
            (Utilities|Array|Add (LocalVariables|Getm_Triangles) (|((2*index)+1) _index_3))))
        (:then_2
          ;;[1 1 1] Curve Side
          (for _index_4 (range 1 (+ (Variables|ProceduralMesh|GetResolution) 2))
            (Utilities|Array|Add (LocalVariables|Getm_Triangles) (|(2*index) _index_4))
            (Utilities|Array|Add (LocalVariables|Getm_Triangles) (|((2*index)+1) _index_4))
            (Utilities|Array|Add (LocalVariables|Getm_Triangles) (|((2*index)+3) _index_4))
            (Utilities|Array|Add (LocalVariables|Getm_Triangles) (|(2*index) _index_4))
            (Utilities|Array|Add (LocalVariables|Getm_Triangles) (|((2*index)+3) _index_4))
            (Utilities|Array|Add (LocalVariables|Getm_Triangles) (|((2*index)+2) _index_4))))
        (:then_3
          ;;[1 1 1] Front Side
          (Utilities|Array|Add (LocalVariables|Getm_Triangles) 0)
          (Utilities|Array|Add (LocalVariables|Getm_Triangles) 1)
          (Utilities|Array|Add (LocalVariables|Getm_Triangles) 3)
          (Utilities|Array|Add (LocalVariables|Getm_Triangles) 0)
          (Utilities|Array|Add (LocalVariables|Getm_Triangles) 3)
          (Utilities|Array|Add (LocalVariables|Getm_Triangles) 2))
        (:then_4
          ;;[1 1 1] Left Side
          (Utilities|Array|Add (LocalVariables|Getm_Triangles) (|((2*{492FDB67-48C4-63DF-678A-B19107B6833C})+6)))
          (Utilities|Array|Add (LocalVariables|Getm_Triangles) (|((2*{492FDB67-48C4-63DF-678A-B19107B6833C})+7)))
          (Utilities|Array|Add (LocalVariables|Getm_Triangles) 1)
          (Utilities|Array|Add (LocalVariables|Getm_Triangles) (|((2*{492FDB67-48C4-63DF-678A-B19107B6833C})+6)))
          (Utilities|Array|Add (LocalVariables|Getm_Triangles) 1)
          (Utilities|Array|Add (LocalVariables|Getm_Triangles) 0))))
    (:then_2
      (return (LocalVariables|Getm_UniqueVertices) (LocalVariables|Getm_Triangles)))))