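; Procedural mesh Blueprint that builds a closed, solid staircase from Size and NumberOfSteps, deferring construction to its parent.
; GenerateVerticesAndTriangles computes shared step vertices and indexes front, top and side quads per step, plus one back and one bottom quad.
; ProcessVertices expands these into unshared vertices per triangle corner with sequential indices.
; ProcessUV then maps a full 0–1 square onto each quad.
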(event EventProcessUV
  (Utilities|Array|Clear (Variables|Default|GetRealUVs))
  (for _index (range 1 (|((4*{E047D957-4743-AAA4-7D16-B49AC2B6C73B})+2)))
    (Utilities|Array|Add :TargetArray (Variables|Default|GetRealUVs))
    (Utilities|Array|Add (Variables|Default|GetRealUVs) "(X=0.000000,Y=1.000000)")
    (Utilities|Array|Add (Variables|Default|GetRealUVs) "(X=1.000000,Y=1.000000)")
    (Utilities|Array|Add :TargetArray (Variables|Default|GetRealUVs))
    (Utilities|Array|Add (Variables|Default|GetRealUVs) "(X=1.000000,Y=1.000000)")
    (Utilities|Array|Add (Variables|Default|GetRealUVs) "(X=1.000000,Y=0.000000)")))

(event EventProcessVertices
  (Utilities|Array|Clear (Variables|Default|GetRealVertices))
  (Utilities|Array|Clear (Variables|Default|GetRealTriangles))
  (bind (_unique_vertices _triangles) (CallFunction|GenerateVerticesandTriangles))
  (for (_ _array_index) _triangles
    (Utilities|Array|Add (Variables|Default|GetRealVertices) (Utilities|Array|Get(acopy) _unique_vertices (Utilities|Array|Get(acopy) _triangles _array_index))))
  (for (_ _array_index_2) (Variables|Default|GetRealVertices)
    (Utilities|Array|Add (Variables|Default|GetRealTriangles) _array_index_2)))

(fn ConstructionScript
  (|CallParentFunction))

(fn GenerateVerticesandTriangles
  (bind _size (Variables|ProceduralMesh|GetSize))
  (Utilities|Array|Clear (LocalVariables|Getm_UniqueVertices))
  (Utilities|Array|Clear (LocalVariables|Getm_Triangles))
  (Utilities|FlowControl|Sequence
    (:then_0
      ;[1 1 1] Calculate the size of the steps
      (LocalVariables|SetstepX (.x _size))
      (LocalVariables|SetstepY (/ (.y _size) (Math|Conversions|ToFloat(Integer) (Variables|ProceduralMesh|GetNumberOfSteps))))
      (LocalVariables|SetstepZ (/ (.z _size) (Math|Conversions|ToFloat(Integer) (Variables|ProceduralMesh|GetNumberOfSteps)))))
    (:then_1
      ;[1 1 1] Generate Vertices
      (for _index (range 0 (- (Variables|ProceduralMesh|GetNumberOfSteps) 1))
        (Utilities|Array|Add (LocalVariables|Getm_UniqueVertices) (Math|Vector|MakeVector 0.0 (|(Index*{5C6EC07C-4A0C-755F-DE9D-F8B582195B3E}) (Math|Conversions|ToFloat(Integer) _index)) 0.0))
        (Utilities|Array|Add (LocalVariables|Getm_UniqueVertices) (Math|Vector|MakeVector (LocalVariables|GetstepX) (|(Index*{5C6EC07C-4A0C-755F-DE9D-F8B582195B3E}) (Math|Conversions|ToFloat(Integer) _index)) 0.0))
        (Utilities|Array|Add (LocalVariables|Getm_UniqueVertices) (Math|Vector|MakeVector 0.0 (|(Index*{5C6EC07C-4A0C-755F-DE9D-F8B582195B3E}) (Math|Conversions|ToFloat(Integer) _index)) (|((Index+1)*{F8C6801A-4741-2DB5-7B02-1EBB4C28EE09}) (Math|Conversions|ToFloat(Integer) _index))))
        (Utilities|Array|Add (LocalVariables|Getm_UniqueVertices) (Math|Vector|MakeVector (LocalVariables|GetstepX) (|(Index*{5C6EC07C-4A0C-755F-DE9D-F8B582195B3E}) (Math|Conversions|ToFloat(Integer) _index)) (|((Index+1)*{F8C6801A-4741-2DB5-7B02-1EBB4C28EE09}) (Math|Conversions|ToFloat(Integer) _index))))
        (Utilities|Array|Add (LocalVariables|Getm_UniqueVertices) (Math|Vector|MakeVector 0.0 (|((Index+1)*{5C6EC07C-4A0C-755F-DE9D-F8B582195B3E}) (Math|Conversions|ToFloat(Integer) _index)) (|((Index+1)*{F8C6801A-4741-2DB5-7B02-1EBB4C28EE09}) (Math|Conversions|ToFloat(Integer) _index))))
        (Utilities|Array|Add (LocalVariables|Getm_UniqueVertices) (Math|Vector|MakeVector (LocalVariables|GetstepX) (|((Index+1)*{5C6EC07C-4A0C-755F-DE9D-F8B582195B3E}) (Math|Conversions|ToFloat(Integer) _index)) (|((Index+1)*{F8C6801A-4741-2DB5-7B02-1EBB4C28EE09}) (Math|Conversions|ToFloat(Integer) _index)))))
      (Utilities|Array|Add (LocalVariables|Getm_UniqueVertices) (Math|Vector|MakeVector 0.0 (|({E047D957-4743-AAA4-7D16-B49AC2B6C73B}*{5C6EC07C-4A0C-755F-DE9D-F8B582195B3E})) 0.0))
      (Utilities|Array|Add (LocalVariables|Getm_UniqueVertices) (Math|Vector|MakeVector (LocalVariables|GetstepX) (|({E047D957-4743-AAA4-7D16-B49AC2B6C73B}*{5C6EC07C-4A0C-755F-DE9D-F8B582195B3E})) 0.0)))
    (:then_2
      ;[1 1 1] Generate triangles
      (for _index_2 (range 0 (- (Variables|ProceduralMesh|GetNumberOfSteps) 1))
        (Utilities|FlowControl|Sequence
          (:then_0
            ;;[1 1 1] Front quad
            (Utilities|Array|Add (LocalVariables|Getm_Triangles) (|(6*Index) _index_2))
            (Utilities|Array|Add (LocalVariables|Getm_Triangles) (|((6*Index)+2) _index_2))
            (Utilities|Array|Add (LocalVariables|Getm_Triangles) (|((6*Index)+3) _index_2))
            (Utilities|Array|Add (LocalVariables|Getm_Triangles) (|(6*Index) _index_2))
            (Utilities|Array|Add (LocalVariables|Getm_Triangles) (|((6*Index)+3) _index_2))
            (Utilities|Array|Add (LocalVariables|Getm_Triangles) (|((6*Index)+1) _index_2)))
          (:then_1
            ;;[1 1 1] Top quad
            (Utilities|Array|Add (LocalVariables|Getm_Triangles) (|((6*Index)+2) _index_2))
            (Utilities|Array|Add (LocalVariables|Getm_Triangles) (|((6*Index)+4) _index_2))
            (Utilities|Array|Add (LocalVariables|Getm_Triangles) (|((6*Index)+5) _index_2))
            (Utilities|Array|Add (LocalVariables|Getm_Triangles) (|((6*Index)+2) _index_2))
            (Utilities|Array|Add (LocalVariables|Getm_Triangles) (|((6*Index)+5) _index_2))
            (Utilities|Array|Add (LocalVariables|Getm_Triangles) (|((6*Index)+3) _index_2)))
          (:then_2
            ;;[1 1 1] Right quad
            (Utilities|Array|Add (LocalVariables|Getm_Triangles) (|((6*Index)+6) _index_2))
            (Utilities|Array|Add (LocalVariables|Getm_Triangles) (|((6*Index)+4) _index_2))
            (Utilities|Array|Add (LocalVariables|Getm_Triangles) (|((6*Index)+2) _index_2))
            (Utilities|Array|Add (LocalVariables|Getm_Triangles) (|((6*Index)+6) _index_2))
            (Utilities|Array|Add (LocalVariables|Getm_Triangles) (|((6*Index)+2) _index_2))
            (Utilities|Array|Add (LocalVariables|Getm_Triangles) (|(6*Index) _index_2)))
          (:then_3
            ;;[1 1 1] Left quad
            (Utilities|Array|Add (LocalVariables|Getm_Triangles) (|((6*Index)+1) _index_2))
            (Utilities|Array|Add (LocalVariables|Getm_Triangles) (|((6*Index)+3) _index_2))
            (Utilities|Array|Add (LocalVariables|Getm_Triangles) (|((6*Index)+5) _index_2))
            (Utilities|Array|Add (LocalVariables|Getm_Triangles) (|((6*Index)+1) _index_2))
            (Utilities|Array|Add (LocalVariables|Getm_Triangles) (|((6*Index)+5) _index_2))
            (Utilities|Array|Add (LocalVariables|Getm_Triangles) (|((6*Index)+7) _index_2))))))
    (:then_3
      ;;[1 1 1] Back quad
      (Utilities|Array|Add (LocalVariables|Getm_Triangles) (|((6*{E047D957-4743-AAA4-7D16-B49AC2B6C73B})+1)))
      (Utilities|Array|Add (LocalVariables|Getm_Triangles) (|((6*{E047D957-4743-AAA4-7D16-B49AC2B6C73B})-1)))
      (Utilities|Array|Add (LocalVariables|Getm_Triangles) (|((6*{E047D957-4743-AAA4-7D16-B49AC2B6C73B})-2)))
      (Utilities|Array|Add (LocalVariables|Getm_Triangles) (|((6*{E047D957-4743-AAA4-7D16-B49AC2B6C73B})+1)))
      (Utilities|Array|Add (LocalVariables|Getm_Triangles) (|((6*{E047D957-4743-AAA4-7D16-B49AC2B6C73B})-2)))
      (Utilities|Array|Add (LocalVariables|Getm_Triangles) (|(6*{E047D957-4743-AAA4-7D16-B49AC2B6C73B}))))
    (:then_4
      ;;[1 1 1] Bottom quad
      (Utilities|Array|Add (LocalVariables|Getm_Triangles) 1)
      (Utilities|Array|Add (LocalVariables|Getm_Triangles) (|((6*{E047D957-4743-AAA4-7D16-B49AC2B6C73B})+1)))
      (Utilities|Array|Add (LocalVariables|Getm_Triangles) (|(6*{E047D957-4743-AAA4-7D16-B49AC2B6C73B})))
      (Utilities|Array|Add (LocalVariables|Getm_Triangles) 1)
      (Utilities|Array|Add (LocalVariables|Getm_Triangles) (|(6*{E047D957-4743-AAA4-7D16-B49AC2B6C73B})))
      (Utilities|Array|Add (LocalVariables|Getm_Triangles) 0))
    (:then_5
      (return (LocalVariables|Getm_UniqueVertices) (LocalVariables|Getm_Triangles)))))