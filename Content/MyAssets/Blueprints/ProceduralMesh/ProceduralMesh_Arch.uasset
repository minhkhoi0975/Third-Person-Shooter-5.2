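; Procedural mesh Blueprint that builds a solid arch segment from inner and outer radius, height, sweep angle and resolution.
; GenerateVerticesAndTriangles rotates four corner points per angular step, then indexes quads for bottom, top, both curves and two end caps.
; ProcessVertices unrolls these into unshared per-triangle vertices with sequential indices, and ProcessUV maps every quad to the unit square in matching face order.
; The construction script only calls its parent.
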(event EventProcessUV
  (Utilities|Array|Clear (Variables|Default|GetRealUVs))
  ;[1 1 1] Generate UVs
  (Utilities|FlowControl|Sequence
    (:then_0
      ;;[1 1 1] Bottom
      (for _index (range 1 (Variables|ProceduralMesh|GetResolution))
        (Utilities|Array|Add :TargetArray (Variables|Default|GetRealUVs))
        (Utilities|Array|Add (Variables|Default|GetRealUVs) "(X=0.000000,Y=1.000000)")
        (Utilities|Array|Add (Variables|Default|GetRealUVs) "(X=1.000000,Y=1.000000)")
        (Utilities|Array|Add (Variables|Default|GetRealUVs) "(X=0.000000,Y=0.000000)")
        (Utilities|Array|Add (Variables|Default|GetRealUVs) "(X=1.000000,Y=1.000000)")
        (Utilities|Array|Add (Variables|Default|GetRealUVs) "(X=1.000000,Y=0.000000)")))
    (:then_1
      ;;[1 1 1] Top
      (for _index_2 (range 1 (Variables|ProceduralMesh|GetResolution))
        (Utilities|Array|Add :TargetArray (Variables|Default|GetRealUVs))
        (Utilities|Array|Add (Variables|Default|GetRealUVs) "(X=0.000000,Y=1.000000)")
        (Utilities|Array|Add (Variables|Default|GetRealUVs) "(X=1.000000,Y=1.000000)")
        (Utilities|Array|Add (Variables|Default|GetRealUVs) "(X=0.000000,Y=0.000000)")
        (Utilities|Array|Add (Variables|Default|GetRealUVs) "(X=1.000000,Y=1.000000)")
        (Utilities|Array|Add (Variables|Default|GetRealUVs) "(X=1.000000,Y=0.000000)")))
    (:then_2
      ;;[1 1 1] Inner Curve
      (for _index_3 (range 1 (Variables|ProceduralMesh|GetResolution))
        (Utilities|Array|Add :TargetArray (Variables|Default|GetRealUVs))
        (Utilities|Array|Add (Variables|Default|GetRealUVs) "(X=0.000000,Y=1.000000)")
        (Utilities|Array|Add (Variables|Default|GetRealUVs) "(X=1.000000,Y=1.000000)")
        (Utilities|Array|Add (Variables|Default|GetRealUVs) "(X=0.000000,Y=0.000000)")
        (Utilities|Array|Add (Variables|Default|GetRealUVs) "(X=1.000000,Y=1.000000)")
        (Utilities|Array|Add (Variables|Default|GetRealUVs) "(X=1.000000,Y=0.000000)")))
    (:then_3
      ;;[1 1 1] Outter Curve
      (for _index_4 (range 1 (Variables|ProceduralMesh|GetResolution))
        (Utilities|Array|Add :TargetArray (Variables|Default|GetRealUVs))
        (Utilities|Array|Add (Variables|Default|GetRealUVs) "(X=0.000000,Y=1.000000)")
        (Utilities|Array|Add (Variables|Default|GetRealUVs) "(X=1.000000,Y=1.000000)")
        (Utilities|Array|Add (Variables|Default|GetRealUVs) "(X=0.000000,Y=0.000000)")
        (Utilities|Array|Add (Variables|Default|GetRealUVs) "(X=1.000000,Y=1.000000)")
        (Utilities|Array|Add (Variables|Default|GetRealUVs) "(X=1.000000,Y=0.000000)")))
    (:then_4
      ;;[1 1 1] Back Side
      (Utilities|Array|Add :TargetArray (Variables|Default|GetRealUVs))
      (Utilities|Array|Add (Variables|Default|GetRealUVs) "(X=0.000000,Y=1.000000)")
      (Utilities|Array|Add (Variables|Default|GetRealUVs) "(X=1.000000,Y=1.000000)")
      (Utilities|Array|Add (Variables|Default|GetRealUVs) "(X=0.000000,Y=0.000000)")
      (Utilities|Array|Add (Variables|Default|GetRealUVs) "(X=1.000000,Y=1.000000)")
      (Utilities|Array|Add (Variables|Default|GetRealUVs) "(X=1.000000,Y=0.000000)"))
    (:then_5
      ;;[1 1 1] Front Side
      (Utilities|Array|Add :TargetArray (Variables|Default|GetRealUVs))
      (Utilities|Array|Add (Variables|Default|GetRealUVs) "(X=0.000000,Y=1.000000)")
      (Utilities|Array|Add (Variables|Default|GetRealUVs) "(X=1.000000,Y=1.000000)")
      (Utilities|Array|Add (Variables|Default|GetRealUVs) "(X=0.000000,Y=0.000000)")
      (Utilities|Array|Add (Variables|Default|GetRealUVs) "(X=1.000000,Y=1.000000)")
      (Utilities|Array|Add (Variables|Default|GetRealUVs) "(X=1.000000,Y=0.000000)"))))

(event EventProcessVertices
  (Utilities|Array|Clear (Variables|Default|GetRealVertices))
  (Utilities|Array|Clear (Variables|Default|GetRealTriangles))
  (bind (_unique_vertices _triangles) (CallFunction|GenerateVerticesandTriangles))
  (for (_ _array_index) _triangles
    (Utilities|Array|Add (Variables|Default|GetRealVertices) (Utilities|Array|Get(acopy) _unique_vertices (Utilities|Array|Get(acopy) _triangles _array_index))))
  (for (_ _array_index_2) (Variables|Default|GetRealVertices)
    (Utilities|Array|Add (Variables|Default|GetRealTriangles) _array_index_2)))

(fn ConstructionScript
  (|CallParentFunction))

(fn GenerateVerticesandTriangles
  (Utilities|Array|Clear (LocalVariables|Getm_UniqueVertices))
  (Utilities|Array|Clear (LocalVariables|Getm_Triangles))
  (Utilities|FlowControl|Sequence
    (:then_0
      ;[1 1 1] Generate Vertices
      (Utilities|FlowControl|Sequence
        (:then_0
          (LocalVariables|SetdAngle (/ (Variables|ProceduralMesh|GetAngle) (Math|Conversions|ToFloat(Integer) (Variables|ProceduralMesh|GetResolution)))))
        (:then_1
          (for _index (range 0 (Variables|ProceduralMesh|GetResolution))
            ;;[1 1 1] Inner Vertices
            (Utilities|Array|Add (LocalVariables|Getm_UniqueVertices) (Math|Conversions|ToVector(Vector2D) (Class|KismetMathLibrary|GetRotated2D (Math|Vector2D|MakeVector2D (Variables|ProceduralMesh|GetInnerRadius) 0.0) (* (LocalVariables|GetdAngle) (Math|Conversions|ToFloat(Integer) _index)))))
            (Utilities|Array|Add (LocalVariables|Getm_UniqueVertices) (Math|Conversions|ToVector(Vector2D) (Class|KismetMathLibrary|GetRotated2D (Math|Vector2D|MakeVector2D (Variables|ProceduralMesh|GetInnerRadius) 0.0) (* (LocalVariables|GetdAngle) (Math|Conversions|ToFloat(Integer) _index))) (Variables|ProceduralMesh|GetHeight)))
            ;;[1 1 1] Outter Vertices
            (Utilities|Array|Add (LocalVariables|Getm_UniqueVertices) (Math|Conversions|ToVector(Vector2D) (Class|KismetMathLibrary|GetRotated2D (Math|Vector2D|MakeVector2D (Variables|ProceduralMesh|GetOutterRadius) 0.0) (* (LocalVariables|GetdAngle) (Math|Conversions|ToFloat(Integer) _index)))))
            (Utilities|Array|Add (LocalVariables|Getm_UniqueVertices) (Math|Conversions|ToVector(Vector2D) (Class|KismetMathLibrary|GetRotated2D (Math|Vector2D|MakeVector2D (Variables|ProceduralMesh|GetOutterRadius) 0.0) (* (LocalVariables|GetdAngle) (Math|Conversions|ToFloat(Integer) _index))) (Variables|ProceduralMesh|GetHeight)))))))
    (:then_1
      ;[1 1 1] Generate Triangles
      (Utilities|FlowControl|Sequence
        (:then_0
          ;;[1 1 1] Bottom
          (for _index_2 (range 1 (Variables|ProceduralMesh|GetResolution))
            (Utilities|Array|Add (LocalVariables|Getm_Triangles) (|((4*Index)-2) _index_2))
            (Utilities|Array|Add (LocalVariables|Getm_Triangles) (|((4*Index)+2) _index_2))
            (Utilities|Array|Add (LocalVariables|Getm_Triangles) (|(4*Index) _index_2))
            (Utilities|Array|Add (LocalVariables|Getm_Triangles) (|((4*Index)-2) _index_2))
            (Utilities|Array|Add (LocalVariables|Getm_Triangles) (|(4*Index) _index_2))
            (Utilities|Array|Add (LocalVariables|Getm_Triangles) (|((4*Index)-4) _index_2))))
        (:then_1
          ;;[1 1 1] Top
          (for _index_3 (range 1 (Variables|ProceduralMesh|GetResolution))
            (Utilities|Array|Add (LocalVariables|Getm_Triangles) (|((4*index)-3) _index_3))
            (Utilities|Array|Add (LocalVariables|Getm_Triangles) (|((4*index)+1) _index_3))
            (Utilities|Array|Add (LocalVariables|Getm_Triangles) (|((4*index)+3) _index_3))
            (Utilities|Array|Add (LocalVariables|Getm_Triangles) (|((4*index)-3) _index_3))
            (Utilities|Array|Add (LocalVariables|Getm_Triangles) (|((4*index)+3) _index_3))
            (Utilities|Array|Add (LocalVariables|Getm_Triangles) (|((4*index)-1) _index_3))))
        (:then_2
          ;;[1 1 1] Inner Curve
          (for _index_4 (range 1 (Variables|ProceduralMesh|GetResolution))
            (Utilities|Array|Add (LocalVariables|Getm_Triangles) (|(4*index) _index_4))
            (Utilities|Array|Add (LocalVariables|Getm_Triangles) (|((4*index)+1) _index_4))
            (Utilities|Array|Add (LocalVariables|Getm_Triangles) (|((4*index)-3) _index_4))
            (Utilities|Array|Add (LocalVariables|Getm_Triangles) (|(4*index) _index_4))
            (Utilities|Array|Add (LocalVariables|Getm_Triangles) (|((4*index)-3) _index_4))
            (Utilities|Array|Add (LocalVariables|Getm_Triangles) (|((4*index)-4) _index_4))))
        (:then_3
          ;;[1 1 1] Outter Curve
          (for _index_5 (range 1 (Variables|ProceduralMesh|GetResolution))
            (Utilities|Array|Add (LocalVariables|Getm_Triangles) (|((4*index)-2) _index_5))
            (Utilities|Array|Add (LocalVariables|Getm_Triangles) (|((4*index)-1) _index_5))
            (Utilities|Array|Add (LocalVariables|Getm_Triangles) (|((4*index)+3) _index_5))
            (Utilities|Array|Add (LocalVariables|Getm_Triangles) (|((4*index)-2) _index_5))
            (Utilities|Array|Add (LocalVariables|Getm_Triangles) (|((4*index)+3) _index_5))
            (Utilities|Array|Add (LocalVariables|Getm_Triangles) (|((4*index)+2) _index_5))))
        (:then_4
          ;;[1 1 1] Back Side
          (Utilities|Array|Add (LocalVariables|Getm_Triangles) (|((4*{DFA98BFE-49E7-D2E3-928D-479A2DBB19DD})+2)))
          (Utilities|Array|Add (LocalVariables|Getm_Triangles) (|((4*{DFA98BFE-49E7-D2E3-928D-479A2DBB19DD})+3)))
          (Utilities|Array|Add (LocalVariables|Getm_Triangles) (|((4*{DFA98BFE-49E7-D2E3-928D-479A2DBB19DD})+1)))
          (Utilities|Array|Add (LocalVariables|Getm_Triangles) (|((4*{DFA98BFE-49E7-D2E3-928D-479A2DBB19DD})+2)))
          (Utilities|Array|Add (LocalVariables|Getm_Triangles) (|((4*{DFA98BFE-49E7-D2E3-928D-479A2DBB19DD})+1)))
          (Utilities|Array|Add (LocalVariables|Getm_Triangles) (|(4*{DFA98BFE-49E7-D2E3-928D-479A2DBB19DD}))))
        (:then_5
          ;;[1 1 1] Front Side
          (Utilities|Array|Add (LocalVariables|Getm_Triangles) 0)
          (Utilities|Array|Add (LocalVariables|Getm_Triangles) 1)
          (Utilities|Array|Add (LocalVariables|Getm_Triangles) 3)
          (Utilities|Array|Add (LocalVariables|Getm_Triangles) 0)
          (Utilities|Array|Add (LocalVariables|Getm_Triangles) 3)
          (Utilities|Array|Add (LocalVariables|Getm_Triangles) 2))))
    (:then_2
      (return (LocalVariables|Getm_UniqueVertices) (LocalVariables|Getm_Triangles)))))