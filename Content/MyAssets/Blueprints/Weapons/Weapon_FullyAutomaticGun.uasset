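; Fully automatic gun weapon Blueprint that keeps firing line-trace shots while the trigger is held.
; StartFiring fires immediately, then runs a looping timer at FireRate that calls FireAutomatic; StopFiring clears that timer.
; Each shot is skipped while reloading, otherwise it spends one ammo and applies recoil and camera shake to the carrying character, or triggers Reload when empty.
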(event `self.StartFiring`
  ;[1 1 1] Start Firing
  (`parent.StartFiring`)
  (`self.FireAutomatic`)
  (bind _returnvalue (`KismetSystemLibrary.K2_SetTimer` null "FireAutomatic" (`self.FireRate`) true))
  (set `self.GunTimer` _returnvalue))

(event `self.StopFiring`
  ;[1 1 1] Stop Firing
  (`parent.StopFiring`)
  (`KismetSystemLibrary.K2_ClearAndInvalidateTimerHandle` (`self.GunTimer`)))

(event `FireAutomatic`
  (bind _carryingcharacter (`self.CarryingCharacter`))
  ;[1 1 1] Fire in fully automatic mode
  (if (not (`self.IsReloading`))
    (if (> (`self.AmmoCount`) 0)
      (`self.FireUsingLineTrace`)
      (`/Engine/EditorBlueprintResources/StandardMacros.IsValid` _carryingcharacter
        (:`Is Valid`
          (`/Game/MyAssets/Blueprints/Characters/Character_Base.RecoilAndShake` _carryingcharacter 0.3 (`self.Recoil`)))
        (:`Is Not Valid`
          _))
      (set `self.AmmoCount` (- (`self.AmmoCount`) 1))
      (else
        (`self.Reload`)))))

(fn `UserConstructionScript`
  (`parent.UserConstructionScript`))