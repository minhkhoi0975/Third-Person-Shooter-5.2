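; Knife weapon that swaps shooting for a melee swing and overrides reload to do nothing.
; Firing runs the parent logic, then plays the attack montage on the carrying character's mesh.
; A separate MeleeAttack event sphere-traces along the blade between the Muzzle and Guard components on the server only.
; It applies generic damage to the hit actor, sparing friendly characters; an ApplyPointDamage node is left unconnected.
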(event `self.StartFiring`
  ;[1 1 1] Firing
  (`parent.StartFiring`)
  (`self.PlayAttackMontage`))

(event `PlayAttackMontage`
  ;[1 1 1] Firing
  (`AnimInstance.Montage_Play` (`SkeletalMeshComponent.GetAnimInstance` (`Character.Mesh` (`self.CarryingCharacter`))) "/Game/MyAssets/Art/Animation/ExperimentalAnimations/Knife/Attack_Knife_Montage.Attack_Knife_Montage" 1.0 "MontageLength" 0.0 false))

(event `self.Reload`)

(event `MeleeAttack`
  (bind _carryingcharacter (`self.CarryingCharacter`))
  ;[1 1 1] Sphere trace to check if the knife hits anything
  (if (and (`KismetSystemLibrary.IsServer`) (`KismetSystemLibrary.IsValid` (`self.CarryingCharacter`)))
    (bind (_outhit _returnvalue) (`KismetSystemLibrary.SphereTraceSingle` (`SceneComponent.K2_GetComponentLocation` (`self.Muzzle`)) (`SceneComponent.K2_GetComponentLocation` (`self.Guard`)) (`self.Blade Radius`) "TraceTypeQuery1"))
    (if _returnvalue
      (bind (_bblockinghit _binitialoverlap _time _distance _location _impactpoint _normal _impactnormal _physmat _hitactor _hitcomponent _hitbonename _bonename _hititem _elementindex _faceindex _tracestart) (`GameplayStatics.BreakHitResult` _outhit))
      (bind _ascharacter_base (cast `/Game/MyAssets/Blueprints/Characters/Character_Base` _hitactor)
        (:`then`
          (if (not (`/Game/MyAssets/Blueprints/Characters/Character_Base.IsOtherCharacterFriend` _ascharacter_base _carryingcharacter))
            (`GameplayStatics.ApplyDamage` _hitactor (`self.Damage`) (`Pawn.GetController` _carryingcharacter) :!label _label)))
        (:`CastFailed`
          (goto _label))))))

(fn `UserConstructionScript`
  (`parent.UserConstructionScript`))