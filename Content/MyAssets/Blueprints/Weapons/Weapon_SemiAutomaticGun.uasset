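; Semi-automatic gun weapon Blueprint that extends a parent weapon's StartFiring to fire one shot per trigger press.
; When not reloading and ammo remains, it fires a line trace, applies recoil and camera shake to the carrying character, then decrements ammo.
; An empty magazine triggers a reload instead of firing.
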(event `self.StartFiring`
  (bind _carryingcharacter (`self.CarryingCharacter`))
  ;[1 1 1] Firing
  (`parent.StartFiring`)
  (if (not (`self.IsReloading`))
    (if (> (`self.AmmoCount`) 0)
      (`self.FireUsingLineTrace`)
      (`/Engine/EditorBlueprintResources/StandardMacros.IsValid` _carryingcharacter
        (:`Is Valid`
          (`/Game/MyAssets/Blueprints/Characters/Character_Base.RecoilAndShake` _carryingcharacter 0.1 (`self.Recoil`)))
        (:`Is Not Valid`
          _))
      (set `self.AmmoCount` (- (`self.AmmoCount`) 1))
      (else
        (`self.Reload`)))))

(fn `UserConstructionScript`
  (`parent.UserConstructionScript`))