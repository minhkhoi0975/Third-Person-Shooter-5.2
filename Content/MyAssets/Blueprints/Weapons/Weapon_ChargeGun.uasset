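; A chargeable gun Blueprint that builds charge while firing is held and launches a projectile on release or automatically at full charge.
; The ChargeWeapon timeline drives CurrentCharge, with play rates set by charge and decharge times, reversing on stop.
; Shots need a minimum charge and a living carrier, aim via player or NPC fallback, and scale damage and initial speed by charge.
; Each shot attempt above that minimum costs one ammo; firing while empty reloads.
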(event `self.StartFiring`
  (`parent.StartFiring`)
  (if (> (`self.AmmoCount`) 0)
    (if (and (not (`self.IsCharging`)) (<= (`self.CurrentCharge`) 0.2))
      (set `self.IsCharging` true)
      (`TimelineComponent.SetPlayRate` (`self.Charge Weapon`) (/ 1.0 (`self.ChargeTime`)))
      (bind (_direction _weapon_charge) (`Timeline|Charge Weapon` :!label _label)
        (:`Update`
          (bind _output_get (set `self.CurrentCharge` (`KismetMathLibrary.FClamp` _weapon_charge)))
          (if (>= _output_get 1.0)
            (`self.StopFiring`)))))
    (else
      (`self.Reload`))))

(event `self.StopFiring`
  (`parent.StopFiring`)
  (if (and (`self.IsCharging`) (>= (`self.CurrentCharge`) 0.2))
    (`self.FireProjectile`)
    (set `self.AmmoCount` (- (`self.AmmoCount`) 1)))
  (set `self.IsCharging` false)
  (`TimelineComponent.SetPlayRate` (`self.Charge Weapon`) (/ 1.0 (`self.DechargeTime`)))
  (goto _label :!via `Reverse`))

(event `self.FireProjectile`
  (bind _carryingcharacter (`self.CarryingCharacter`))
  (bind _audio (`self.Audio`))
  (bind _returnvalue (`SceneComponent.K2_GetComponentLocation` (`self.Muzzle`)))
  ;[1 1 1] Firing
  ;;[1 1 1] A gun cannot fire if there is no carrier, or the carrier is dead.
  (if (and (`KismetSystemLibrary.IsValid` _carryingcharacter) (`/Game/MyAssets/Blueprints/Characters/Character_Base.IsAlive` _carryingcharacter))
    (`|ExecutionSequence`
      (:`then_0`
        ;;[1 1 1] Find the Firing Direction
        (bind (_direction _iscontrollervalid_) (`self.FindFiringDirectionForPlayer`))
        (set `self.FiringDirection` _direction)
        (if (not _iscontrollervalid_)
          (bind _direction_2 (`self.FindFiringDirectionForNPC`))
          (set `self.FiringDirection` _direction_2)))
      (:`then_1`
        ;;[1 1 1] Spawn a projectile.
        (bind _returnvalue_2 (`|SpawnActorFromClass` (`self.Projectile`) (`KismetMathLibrary.MakeTransform` _returnvalue (`KismetMathLibrary.FindLookAtRotation` _returnvalue (+ _returnvalue (`self.FiringDirection`))) (0.5 0.5 0.5)) "AdjustIfPossibleButDontSpawnIfColliding" "SelectDefaultAtRuntime" null (* (`self.Damage`) (`self.CurrentCharge`)) (`self.BulletHoleMaterial`) (`self.BulletHoleScale`) (`self.BulletHoleParticleEffect`) (`self.CarryingCharacter`)))
        (bind _projectile (`/Game/MyAssets/Blueprints/Weapons/Projectiles/Projectile_Base.Projectile` _returnvalue_2)
          (:`then`
            (set `ProjectileMovementComponent.InitialSpeed` (* (`ProjectileMovementComponent.InitialSpeed` _projectile) (`self.CurrentCharge`)) _projectile))
          (:`else`)))
      (:`then_2`
        ;;[1 1 1] Play the shooting sound.
        (`AudioComponent.Stop` _audio)
        (`AudioComponent.Play` _audio 0.0)))))

(fn `UserConstructionScript`
  (`parent.UserConstructionScript`))