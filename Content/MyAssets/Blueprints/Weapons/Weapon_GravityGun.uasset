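; Gravity gun weapon that picks up, carries, drops and launches physics-simulated objects.
; Secondary action toggles between dropping and grabbing, using a visibility line trace from the muzzle and a PhysicsHandle.
; Tick moves the handle target to HeldObjectLocation to carry the object.
; Firing releases any held object and applies a velocity-change impulse along the carrying character's camera forward, while Reload is overridden to do nothing.
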(event `AttractObject`
  (bind _returnvalue (`SceneComponent.K2_GetComponentLocation` (`self.Muzzle`)))
  ;[1 1 1] Pick up an object.
  (bind _direction (`self.FindFiringDirectionForPlayer`))
  (bind (_outhit _returnvalue_2) (`KismetSystemLibrary.LineTraceSingle` _returnvalue (+ _returnvalue _direction) "TraceTypeQuery1"))
  (if _returnvalue_2
    (bind (_bblockinghit _binitialoverlap _time _distance _location _impactpoint _normal _impactnormal _physmat _hitactor _hitcomponent) (`GameplayStatics.BreakHitResult` _outhit))
    (if (`SceneComponent.IsSimulatingPhysics` _hitcomponent "None")
      (`PhysicsHandleComponent.GrabComponentAtLocationWithRotation` :`self` (`self.PhysicsHandle`) :`Component` _hitcomponent :`Location` (`SceneComponent.K2_GetComponentLocation` _hitcomponent))
      (set `self.IsHoldingObject` true))))

(event `LaunchObject`
  ;[1 1 1] Launch the object.
  (if (`self.IsHoldingObject`)
    (`self.DropObject`)
    (`PrimitiveComponent.AddImpulse` (`.HitComponent` (`GameplayStatics.BreakHitResult` (stale `AttractObject` _outhit))) (* (`KismetMathLibrary.Normal` (`SceneComponent.GetForwardVector` (`/Game/MyAssets/Blueprints/Characters/Character_Base.Camera` (`self.CarryingCharacter`)))) (`self.LaunchVelocity`)) "None" true)))

(event `DropObject`
  ;[1 1 1] Drop an object.
  (`PhysicsHandleComponent.ReleaseComponent` (`self.PhysicsHandle`))
  (set `self.IsHoldingObject` false))

(event `self.ReceiveTick`
  (params (DeltaSeconds :type "Float (single-precision)"))
  ;[1 1 1] Update Held Object
  (`PhysicsHandleComponent.SetTargetLocation` (`self.PhysicsHandle`) (`SceneComponent.K2_GetComponentLocation` (`self.HeldObjectLocation`))))

(event `self.StartFiring`
  (`parent.StartFiring`)
  (`self.LaunchObject`))

(event `self.StartPerformingSecondaryAction`
  (`parent.StartPerformingSecondaryAction`)
  (if (`self.IsHoldingObject`)
    (`self.DropObject`)
    (else
      (`self.AttractObject`))))

(event `self.Reload`)

(fn `UserConstructionScript`
  (`parent.UserConstructionScript`))