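; Grenade launcher weapon Blueprint that fires projectile actors when its carrier shoots.
; Firing is blocked while reloading, triggers a reload when empty, and otherwise spawns a projectile, applies recoil and camera shake, and consumes ammo.
; Projectiles launch from the muzzle along a player aim direction, falling back to NPC aiming without a valid controller, then a multicast plays the shot sound.
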(event `self.StartFiring`
  (bind _carryingcharacter (`self.CarryingCharacter`))
  ;[1 1 1] Firing
  (`parent.StartFiring`)
  (if (not (`self.IsReloading`))
    (if (> (`self.AmmoCount`) 0)
      (`self.SpawnProjectile`)
      (`/Engine/EditorBlueprintResources/StandardMacros.IsValid` _carryingcharacter
        (:`Is Valid`
          (`/Game/MyAssets/Blueprints/Characters/Character_Base.RecoilAndShake` _carryingcharacter 0.1 (`self.Recoil`)))
        (:`Is Not Valid`
          _))
      (set `self.AmmoCount` (- (`self.AmmoCount`) 1))
      (else
        (`self.Reload`)))))

(event `SpawnProjectile`
  (bind _carryingcharacter (`self.CarryingCharacter`))
  (bind _returnvalue (`SceneComponent.K2_GetComponentLocation` (`self.Muzzle`)))
  ;[1 1 1] Firing
  ;;[1 1 1] A gun cannot fire if there is no carrier, or the carrier is dead.
  (if (and (`KismetSystemLibrary.IsValid` _carryingcharacter) (`/Game/MyAssets/Blueprints/Characters/Character_Base.IsAlive` _carryingcharacter))
    (`|ExecutionSequence`
      (:`then_0`
        ;;[1 1 1] Find the Firing Direction
        (bind (_direction _iscontrollervalid_) (`self.FindFiringDirectionForPlayer`))
        (set `self.FiringDirection` _direction)
        (if (not _iscontrollervalid_)
          (bind _direction_2 (`self.FindFiringDirectionForNPC`))
          (set `self.FiringDirection` _direction_2)))
      (:`then_1`
        ;;[1 1 1] Spawn a projectile.
        (`|SpawnActorFromClass` (`self.Projectile`) (`KismetMathLibrary.MakeTransform` _returnvalue (`KismetMathLibrary.FindLookAtRotation` _returnvalue (+ _returnvalue (`self.FiringDirection`)))) "AlwaysSpawn" "SelectDefaultAtRuntime" null (`self.Damage`) "/Game/MyAssets/Art/Textures/bullet_hole_material.bullet_hole_material" (5.0 5.0 5.0) "/Game/ThirdPartyAssets/TomLooman/ParticleEffects/Weapons/WeaponEffects/GenericImpact/P_RifleImpact.P_RifleImpact" (`self.CarryingCharacter`)))
      (:`then_2`
        ;;[1 1 1] Play the shooting sound.
        (`self.PlayShootingSoundMulticast`)))))

(fn `UserConstructionScript`
  (`parent.UserConstructionScript`))