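; Gatling gun weapon that must spin up before firing automatic line-trace shots, extending a parent weapon's start and stop firing logic.
; A timeline drives CurrentCharge at rates derived from ChargeTime and DechargeTime, starting a looping fire timer at full charge and reversing on stop.
; Each timer tick fires, applies recoil and shake to the carrier and decrements ammo, or reloads and restarts the charge when empty.
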(event Custom|FireAutomatic
  (bind _carryingcharacter (Variables|Default|GetCarryingCharacter))
  ;[1 1 1] Fire in fully automatic mode
  (if (not (Variables|Default|GetIsReloading))
    (if (> (Variables|Default|GetAmmoCount) 0)
      (if (>= (Variables|Default|GetCurrentCharge) 1.0)
        (CallFunction|FireUsingLineTrace)
        (Utilities|IsValid _carryingcharacter
          (:Is%20Valid
            (Default|RecoilandShake _carryingcharacter 0.3 (Variables|Default|GetRecoil))
            (Variables|Default|SetAmmoCount (|({98B005B7-40B4-8B60-9190-958C1E0BBAD5}-1))))))
      (else
        (CallFunction|Reload)
        (Components|Timeline|SetNewTime (Variables|Default|GetChargeUpGun) 0.0)
        ;[1 1 1] Start Firing
        (bind _charge (Timeline|ChargeUpGun Play)
          (:Update
            (bind _output_get (Variables|Default|SetCurrentCharge (Math|Float|Lerp 0.0 1.0 _charge)))
            (if (>= _output_get 1.0)
              (bind _returnvalue (Utilities|Time|SetTimerbyFunctionName 0 "FireAutomatic" (Variables|Default|GetFireRate) true))
              (Variables|Default|SetGunTimer _returnvalue))))))))

(event EventStopFiring
  ;[1 1 1] Stop Firing
  (|CallParentFunction)
  (Utilities|Time|ClearandInvalidateTimerbyHandle (Variables|Default|GetGunTimer))
  (Components|Timeline|SetPlayRate (Variables|Default|GetChargeUpGun) (|(1/{A86F2659-408D-0B60-C558-43AC607C5BF0})))
  ;[1 1 1] Start Firing
  (bind _charge (Timeline|ChargeUpGun Reverse)
    (:Update
      (bind _output_get (Variables|Default|SetCurrentCharge (Math|Float|Lerp 0.0 1.0 _charge)))
      (if (>= _output_get 1.0)
        (bind _returnvalue (Utilities|Time|SetTimerbyFunctionName 0 "FireAutomatic" (Variables|Default|GetFireRate) true))
        (Variables|Default|SetGunTimer _returnvalue)))))

(event EventStartFiring
  ;[1 1 1] Start Firing
  (|CallParentFunction)
  (Components|Timeline|SetPlayRate (Variables|Default|GetChargeUpGun) (|(1/{95F2AE5E-4D35-9926-9BD5-AD8FE9702DED})))
  (bind _charge (Timeline|ChargeUpGun Play)
    (:Update
      (bind _output_get (Variables|Default|SetCurrentCharge (Math|Float|Lerp 0.0 1.0 _charge)))
      (if (>= _output_get 1.0)
        (bind _returnvalue (Utilities|Time|SetTimerbyFunctionName 0 "FireAutomatic" (Variables|Default|GetFireRate) true))
        (Variables|Default|SetGunTimer _returnvalue)))))

(fn ConstructionScript
  (|CallParentFunction))