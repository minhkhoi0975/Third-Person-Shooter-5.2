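; Base weapon actor that tracks firing, secondary-action and ammo state, scales reload montages to reload time, and provides hitscan firing.
; Players trace from the camera; AI traces from the muzzle toward its focus actor, with spread.
; Hits damage non-friendly characters, push physics objects and leave bullet holes.
; Each shot also plays sound and muzzle flash, reports AI noise and spawns a zero-damage projectile as tracer, mirrored on clients.
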(event Custom|StartFiring
  (Variables|Default|SetIsFiring true))

(event Custom|StartPerformingSecondaryAction
  (Variables|Default|SetIsPerformingSecondaryAction true))

(event Custom|StopPerformingSecondaryAction
  (Variables|Default|SetIsPerformingSecondaryAction false))

(event Custom|Reload
  ;[1 1 1] Reloading
  (bind _carryingcharacter (Variables|Default|GetCarryingCharacter)
    (:then
      (bind _can_reload_ (Default|CanReload _carryingcharacter))
      (if _can_reload_
        (CallFunction|PlayReloadAnimationMontage)))
    (:else)))

(event Custom|PlayReloadAnimationMontage
  ;[1 1 1] Reloading
  (bind _carryingcharacter (Variables|Default|GetCarryingCharacter)
    (:then
      (if (not (Variables|/Game/MyAssets/Blueprints/Characters/Character_Base.Character_Base_C|GetbReloading _carryingcharacter))
        (bind _returnvalue (Animation|Montage|MontagePlay (Components|SkeletalMesh|GetAnimInstance (Variables|/Script/Engine.Character|GetMesh _carryingcharacter)) "/Game/MyAssets/Art/Animation/Reloading/Reload_Montage.Reload_Montage" 1.0 "MontageLength" 0.0 true))
        (Animation|Montage|MontageSetPlayRate (Components|SkeletalMesh|GetAnimInstance (Variables|/Script/Engine.Character|GetMesh _carryingcharacter)) "/Game/MyAssets/Art/Animation/Reloading/Reload_Montage.Reload_Montage" (/ _returnvalue (Variables|Stats|GetReloadTime)))))
    (:else)))

(event Custom|StopFiring
  (Variables|Default|SetIsFiring false))

(event EventBeginPlay
  (Variables|Stats|SetAmmoCount (Variables|Stats|GetAmmoMax)))

(event Custom|SpawnMuzzleFlash
  (bind _mesh (Variables|Default|GetMesh))
  ;[1 1 1] Spawn Muzzle Flash
  (Effects|SpawnEmitterAttached (Variables|MuzzleFlash|GetMuzzleFlashParticleEffect) (Variables|Default|GetMuzzle) "None" (Transformation|GetSocketLocation _mesh "Muzzle") (Transformation|GetSocketRotation _mesh "Muzzle") (Variables|MuzzleFlash|GetMuzzleFlashScale) "KeepWorldPosition"))

(event Custom|PlayShootingSoundMulticast
  (bind _audio (Variables|Default|GetAudio))
  ;[1 1 1] Play Shooting Sound
  (Audio|Components|Audio|Stop _audio)
  (Audio|Components|Audio|Play _audio 0.0))

(event Custom|SpawnTraceOnClients
  (params (HitResult :type Hit%20Result%20Structure%20%28by%20ref%29) (Hit :type Boolean))
  ;[1 1 1] Spawn Trace (if the weapon uses line tracing instead of projectiles)
  (Networking|SwitchHasAuthority
    (:Remote
      (CallFunction|SpawnTrace HitResult Hit))))

(event Custom|CreateBulletHoleMulticast
  (params (Hit%20Info :type Hit%20Result%20Structure))
  (bind (_bblockinghit _binitialoverlap _time _distance _location _impactpoint _normal _impactnormal _physmat _hitactor _hitcomponent) (Collision|BreakHitResult Hit%20Info))
  (bind _returnvalue (Math|Rotator|MakeRotfromX _impactnormal))
  ;[1 1 1] Create a Bullet Hole
  (Class|GameplayStatics|SpawnDecalAttached (Variables|BulletHole|GetBulletHoleMaterial) (Variables|BulletHole|GetBulletHoleScale) _hitcomponent "None" _impactpoint _returnvalue "KeepWorldPosition" 8.0)
  (Effects|SpawnEmitteratLocation (Variables|BulletHole|GetBulletHoleParticleEffect) _impactpoint _returnvalue))

(event Custom|SpawnTrace
  (params (HitResult :type Hit%20Result%20Structure%20%28by%20ref%29) (Hit :type Boolean))
  (bind (_bblockinghit _binitialoverlap _time _distance _location _impactpoint _normal _impactnormal _physmat _hitactor _hitcomponent _hitbonename _bonename _hititem _elementindex _faceindex _tracestart _traceend) (Collision|BreakHitResult HitResult))
  (bind _muzzle (Variables|Default|GetMuzzle))
  (bind _returnvalue (Transformation|GetWorldLocation _muzzle))
  ;[1 1 1] Spawn Trace (if the weapon uses line tracing instead of projectiles)
  (Game|SpawnActorfromClass (Variables|Stats|GetProjectile) (Math|Transform|MakeTransform _returnvalue (Math|Rotator|FindLookatRotation _returnvalue (Math|Vector|SelectVector _impactpoint _traceend Hit)) "0.500000,0.500000,0.500000") "AdjustIfPossibleButDontSpawnIfColliding" "SelectDefaultAtRuntime" 0 0.0 "/Game/MyAssets/Art/Textures/bullet_hole_material.bullet_hole_material" "5.000000,5.000000,5.000000" "/Game/ThirdPartyAssets/TomLooman/ParticleEffects/Weapons/WeaponEffects/GenericImpact/P_RifleImpact.P_RifleImpact" (Variables|Default|GetCarryingCharacter)))

(fn ConstructionScript
  (Audio|Components|Audio|SetSound (Variables|Default|GetAudio) (Variables|Sound|GetFiringSound)))

(fn FindFiringDirectionforPlayer
  (bind _carryingcharacter (Variables|Default|GetCarryingCharacter))
  (bind _camera (Variables|/Game/MyAssets/Blueprints/Characters/Character_Base.Character_Base_C|GetCamera _carryingcharacter))
  (bind _returnvalue (Transformation|GetWorldLocation _camera))
  ;[1 1 1] Make sure that this character is controlled by a player.
  (Utilities|Casting|CastToPlayerController (Pawn|GetController _carryingcharacter))
  ;[1 1 1] Line trace from the player's camera to the middle of the screen.
  (bind (_outhit _returnvalue_2) (Collision|LineTraceByChannel _returnvalue (+ _returnvalue (* (Math|Vector|GetForwardVector _camera) 8e+03)) "TraceTypeQuery1" false 0 "None"))
  ;[1 1 1] The line hits an object: Create a vector that points from the gun's muzzle to the impact point.
  (return (- (Math|Vector|SelectVector (.ImpactPoint (Collision|BreakHitResult _outhit)) (.TraceEnd (Collision|BreakHitResult _outhit)) _returnvalue_2) (Transformation|GetWorldLocation (Variables|Default|GetMuzzle))) true))

(fn FindFiringDirectionforNPC
  (bind _asaicontroller (Utilities|Casting|CastToAIController (Pawn|GetController (Variables|Default|GetCarryingCharacter))))
  (if (Utilities|IsValid (Class|AIController|GetFocusActor _asaicontroller))
    (return (- (Transformation|GetActorLocation (Class|AIController|GetFocusActor _asaicontroller)) (Transformation|GetWorldLocation (Variables|Default|GetMuzzle))) true)))

(fn FireUsingLineTrace
  (bind (_outhit _returnvalue) (Firing|LineTrace))
  (Utilities|FlowControl|Sequence
    (:then_0
      ;[0 1 0] Handle Collision
      (if _returnvalue
        (Utilities|FlowControl|Sequence
          (:then_0
            ;;[1 1 1] If the line hits a character, and the character is an enemy, inflict damage to that character.
            (bind _ascharacter_base (Utilities|Casting|CastToCharacter_Base (.HitActor (Collision|BreakHitResult _outhit))))
            (if (not (Default|IsOtherCharacterFriend _ascharacter_base (Variables|Default|GetCarryingCharacter)))
              (Game|Damage|ApplyPointDamage (.HitActor (Collision|BreakHitResult _outhit)) (Variables|Stats|GetDamage) (Math|Vector|Normalize (- (.ImpactPoint (Collision|BreakHitResult _outhit)) (Transformation|GetWorldLocation (Variables|Default|GetMuzzle)))) _outhit (Pawn|GetController (Variables|Default|GetCarryingCharacter)) self)))
          (:then_1
            ;;[1 1 1] Create a bullet hole and impact effect.
            (CallFunction|CreateBulletHoleMulticast _outhit))
          (:then_2
            ;;[1 1 1] If the other component is simulating physics, add impulse to it.
            (if (Physics|IsSimulatingPhysics (.HitComponent (Collision|BreakHitResult _outhit)) "None")
              (Physics|AddImpulseatLocation (.HitComponent (Collision|BreakHitResult _outhit)) (|((HitDirection*{8057D5F6-48BF-D2D0-AA29-6F89527DAA18})*1000) (Math|Vector|Normalize (- (.ImpactPoint (Collision|BreakHitResult _outhit)) (Transformation|GetWorldLocation (Variables|Default|GetMuzzle))))) (.ImpactPoint (Collision|BreakHitResult _outhit)) "None"))))))
    (:then_1
      ;[0 1 0] Play Shooting Sound
      (CallFunction|PlayShootingSoundMulticast)
      (Class|AISenseHearing|ReportNoiseEvent (Transformation|GetActorLocation) 1.0 (Variables|Default|GetCarryingCharacter) 0.0 "Noise"))
    (:then_2
      ;[0.0696 1 0] Spawn Muzzle Flash
      (CallFunction|SpawnMuzzleFlash))
    (:then_3
      ;[0 1 0] Spawn Trace
      (CallFunction|SpawnTrace _outhit _returnvalue)
      (CallFunction|SpawnTraceonClients _outhit _returnvalue))))

(fn LineTracefromCamera
  (bind _carryingcharacter (Variables|Default|GetCarryingCharacter)
    (:then
      (bind (_outhit _return_value) (Default|LineTracefromCamera _carryingcharacter (Variables|Stats|GetProjectileSpread) 1e+06))
      (Development|PrintString "Line trace from camera" false false)
      (return _outhit _return_value))
    (:else)))

(fn LineTracefromMuzzle
  (bind _muzzle (Variables|Default|GetMuzzle))
  (bind _returnvalue (Transformation|GetWorldLocation _muzzle))
  (bind _carryingcharacter (Variables|Default|GetCarryingCharacter)
    (:then
      (bind _asthird_person_character_aicontroller (Utilities|Casting|CastToThirdPersonCharacterAIController (Pawn|GetController _carryingcharacter)))
      (Utilities|IsValid (Class|AIController|GetFocusActor _asthird_person_character_aicontroller)
        (:Is%20Valid
          (bind (_outhit _returnvalue_2) (Collision|LineTraceByChannel _returnvalue (+ _returnvalue (* (Math|Random|RandomUnitVectorinConeinDegrees (Math|Vector|Normalize (- (Transformation|GetActorLocation (Class|AIController|GetFocusActor _asthird_person_character_aicontroller)) _returnvalue)) (* (Variables|Stats|GetProjectileSpread) 2.0)) 1e+06)) "TraceTypeQuery1" false 0 "None" true "(R=1.000000,G=0.000000,B=0.071821,A=1.000000)"))
          (Development|PrintString "Line trace from muzzle" false false)
          (return _outhit _returnvalue_2))))
    (:else)))

(fn LineTrace
  (bind _carryingcharacter (Variables|Default|GetCarryingCharacter)
    (:then
      (Utilities|Casting|CastToThirdPersonCharacterPlayerController (Pawn|GetController _carryingcharacter)
        (:then
          (bind (_outhit _returnvalue) (Firing|LineTracefromCamera))
          (return _outhit _returnvalue))
        (:CastFailed
          (bind (_outhit_2 _returnvalue_2) (Firing|LineTracefromMuzzle))
          (return _outhit_2 _returnvalue_2))))
    (:else
      (Development|PrintString "WARNING: Weapon has invalid CarryingCharacter" false true "(R=1.000000,G=0.000000,B=0.000000,A=1.000000)"))))

(fn IsOutOfAmmo
  (return (<= (Variables|Stats|GetAmmoCount) 0)))