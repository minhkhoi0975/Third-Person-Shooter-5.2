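; Fire is an environmental hazard that deals periodic environmental damage to actors inside its DamageZone.
; On the server, overlap events add and remove actors in DamagedActors, and each new entry sets a looping CauseDamage timer at DamageInterval.
; CauseDamage applies Damage to every valid tracked actor and drops invalid ones.
; The timer is cleared once the list is empty.
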(event `self.DamageZone.OnComponentBeginOverlap`
  (params (OverlappedComponent :type "PrimitiveComponent Object Reference") (OtherActor :type "Actor Object Reference") (OtherComp :type "PrimitiveComponent Object Reference") (OtherBodyIndex :type Integer) (bFromSweep :type Boolean) (SweepResult :type "HitResult Structure (by ref)"))
  (if (`KismetSystemLibrary.IsServer`)
    (if (not (`KismetArrayLibrary.Array_Contains` (`self.DamagedActors`) OtherActor))
      (`KismetArrayLibrary.Array_Add` (`self.DamagedActors`) OtherActor)
      (`KismetSystemLibrary.PrintString` (`KismetStringLibrary.Concat_StrStr` (`KismetSystemLibrary.GetDisplayName` OtherActor) " enters the fire.") false false)
      (`KismetSystemLibrary.K2_SetTimer` null "CauseDamage" (`self.DamageInterval`) true))))

(event `self.DamageZone.OnComponentEndOverlap`
  (params (OverlappedComponent :type "PrimitiveComponent Object Reference") (OtherActor :type "Actor Object Reference") (OtherComp :type "PrimitiveComponent Object Reference") (OtherBodyIndex :type Integer))
  (if (`KismetSystemLibrary.IsServer`)
    (`KismetArrayLibrary.Array_RemoveItem` (`self.DamagedActors`) OtherActor)
    (`KismetSystemLibrary.PrintString` (`KismetStringLibrary.Concat_StrStr` (`KismetSystemLibrary.GetDisplayName` OtherActor) " leaves the fire.") false false)
    (if (== (`KismetArrayLibrary.Array_Length` (`self.DamagedActors`)) 0)
      (`KismetSystemLibrary.K2_ClearTimer` null "CauseDamage"))))

(event `CauseDamage`
  (`|ExecutionSequence`
    (:`then_0`
      (for _array_element (`self.DamagedActors`)
        (`/Engine/EditorBlueprintResources/StandardMacros.IsValid` _array_element
          (:`Is Valid`
            (`GameplayStatics.ApplyDamage` _array_element (`self.Damage`) null self "/Engine/EngineDamageTypes/DmgTypeBP_Environmental.DmgTypeBP_Environmental_C")
            (`KismetSystemLibrary.PrintString` (`KismetStringLibrary.Concat_StrStr` (`KismetSystemLibrary.GetDisplayName` _array_element) " receives " (`KismetStringLibrary.Conv_DoubleToString` (`self.Damage`)) "damage.") false false))
          (:`Is Not Valid`
            (`KismetArrayLibrary.Array_RemoveItem` (`self.DamagedActors`) _array_element)))))
    (:`then_1`
      (if (== (`KismetArrayLibrary.Array_Length` (`self.DamagedActors`)) 0)
        (`KismetSystemLibrary.K2_ClearTimer` null "CauseDamage")))))

(fn `UserConstructionScript`)