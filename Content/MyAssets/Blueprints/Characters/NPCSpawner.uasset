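; NPCSpawner is a placeable actor that periodically spawns AI-controlled NPCs at its own location and rotation.
; On BeginPlay it spawns once, then a looping timer repeats the spawn every WaitTime.
; Each spawn is skipped once 100 actors of the template class exist in the level, counted globally rather than per spawner.
; New NPCs run the configured behavior tree and receive the spawner's PatrolPath through Character_Base.
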(event `self.ReceiveBeginPlay`
  (`self.Spawn`)
  (`KismetSystemLibrary.K2_SetTimerDelegate` (delegate `Spawn`) (`self.WaitTime`) true))

(event `Spawn`
  (bind (_returnvalue_location _returnvalue_rotation) (`KismetMathLibrary.BreakTransform` (`SceneComponent.K2_GetComponentToWorld` (`self.DefaultSceneRoot`))))
  (bind _outactors (`GameplayStatics.GetAllActorsOfClass` (`self.NPC Template`)))
  (if (< (`KismetArrayLibrary.Array_Length` _outactors) 100)
    (bind _returnvalue (`AIBlueprintHelperLibrary.SpawnAIFromClass` (`self.NPC Template`) (`self.Behavior Tree`) _returnvalue_location _returnvalue_rotation true null))
    (bind _ascharacter_base (cast `/Game/MyAssets/Blueprints/Characters/Character_Base` _returnvalue))
    (set `/Game/MyAssets/Blueprints/Characters/Character_Base.PatrolPath` (`self.Patrol Path`) _ascharacter_base)))

(fn `UserConstructionScript`)